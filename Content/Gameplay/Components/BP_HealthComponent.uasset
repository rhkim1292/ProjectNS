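; Health component that tracks the owning actor's health and destroys that actor when it runs out.
; TakeDamage and Heal adjust CurrentHealth, clamped between zero and MaxHealth, and both are ignored once IsDead is set.
; When damage brings health to zero, TakeDamage sets IsDead and calls Die, which destroys the owner immediately.
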(event Custom|TakeDamage
  (params (DamageAmount :type Float%20%28double-precision%29))
  (if (not (Variables|Default|GetbIsDead))
    (bind _output_get (Variables|Default|SetCurrentHealth (Math|Float|Clamp(Float) (- (Variables|Default|GetCurrentHealth) DamageAmount) 0.0 (Variables|Default|GetMaxHealth))))
    (if (<= _output_get 0.0)
      (Variables|Default|SetbIsDead true)
      (CallFunction|Die))))

(event Custom|Die
  (Actor|DestroyActor (Components|GetOwner)))

(event Custom|Heal
  (params (HealAmount :type Float%20%28double-precision%29))
  (if (not (Variables|Default|GetbIsDead))
    (Variables|Default|SetCurrentHealth (Math|Float|Clamp(Float) (+ (Variables|Default|GetCurrentHealth) HealAmount) 0.0 (Variables|Default|GetMaxHealth)))))