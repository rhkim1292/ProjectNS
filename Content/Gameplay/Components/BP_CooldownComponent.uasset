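; Component that tracks named cooldowns for gameplay code to start, query and clear.
; ActiveCooldowns maps each name to its end time in game seconds, which the active and remaining-time queries compare against the current time.
; Tick loops over the map and calls OnCooldownExpired for expired entries.
; Only ClearCooldown removes entries, so the expiry call repeats every tick until the entry is cleared or restarted.
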(event EventTick
  (params (DeltaSeconds :type Float%20%28single-precision%29))
  (bind _keypin (Utilities|Map|ForEachLoop(Map) (Variables|Default|GetActiveCooldowns))
    (:then
      (if (not (CallFunction|IsonCooldown _keypin))
        (Default|CallOnCooldownExpired _keypin)))))

(fn StartCooldown
  (params (CooldownName :type String) (Duration :type Float%20%28double-precision%29))
  (Utilities|Map|Add (Variables|Default|GetActiveCooldowns) CooldownName (+ (Utilities|Time|GetGameTimeinSeconds) Duration)))

(fn IsonCooldown
  (params (CooldownName :type String))
  (bind _activecooldowns (Variables|Default|GetActiveCooldowns))
  (bind (_value _returnvalue) (Utilities|Map|Find _activecooldowns CooldownName))
  (if _returnvalue
    (if (< (Utilities|Time|GetGameTimeinSeconds) _value)
      (return true)
      (else
        (return false)))
    (else
      (return false))))

(fn GetRemainingCooldown
  (params (CooldownName :type String))
  (bind _activecooldowns (Variables|Default|GetActiveCooldowns))
  (bind (_value _returnvalue) (Utilities|Map|Find _activecooldowns CooldownName))
  (if _returnvalue
    (return (Math|Float|Max(Float) (- _value (Utilities|Time|GetGameTimeinSeconds)) 0.0))
    (else
      (return 0.0))))

(fn ClearCooldown
  (params (CooldownName :type String))
  (Utilities|Map|Remove (Variables|Default|GetActiveCooldowns) CooldownName))