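; Base weapon Blueprint for a hitscan gun that attaches to the WeaponSocket of any actor overlapping its pickup radius and notifies that actor.
; TryFire and TryReload gate firing and reloading on state and ammo, with delays setting fire rate and reload time.
; Firing line-traces from player 0's camera with debug drawing, sending damage through BPI_Damageable.
; Shots and reloads broadcast magazine and reserve counts through OnAmmoChanged.
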(event OnComponentBeginOverlap(PickupRadius)
  (params (OverlappedComponent :type Primitive%20Component%20Object%20Reference) (OtherActor :type Actor%20Object%20Reference) (OtherComp :type Primitive%20Component%20Object%20Reference) (OtherBodyIndex :type Integer) (bFromSweep :type Boolean) (SweepResult :type Hit%20Result%20Structure%20%28by%20ref%29))
  (if (not (Variables|Default|GetbIsEquipped))
    (CallFunction|EquipWeapon OtherActor)))

(event Custom|TryFire
  (bind _currentmagazine (Variables|Default|GetCurrentMagazine))
  (if (Math|Boolean|ANDBoolean (Variables|Default|GetbIsEquipped) (Variables|Default|GetbCanFire) (not (Variables|Default|GetbIsReloading)) (> _currentmagazine 0))
    (CallFunction|Fire)
    (elif (<= _currentmagazine 0)
      _)))

(event Custom|EquipWeapon
  (params (EquippingActor :type Actor%20Object%20Reference))
  (Variables|Default|SetbIsEquipped true)
  (Collision|SetCollisionEnabled (Variables|Default|GetWeaponMesh) "NoCollision")
  (Collision|SetCollisionEnabled (Variables|Default|GetPickupRadius) "NoCollision")
  (Transformation|AttachComponentToComponent (Actor|GetComponentbyClass EquippingActor "/Script/Engine.SkeletalMeshComponent") "WeaponSocket" "SnapToTarget" "SnapToTarget" "KeepRelative" true)
  (Class|BPICanEquipWeapon|OnWeaponEquipped(Message) EquippingActor self)
  (Variables|Default|SetCurrentOwner EquippingActor))

(event Custom|Fire
  (bind _returnvalue (Game|GetPlayerCameraManager 0))
  (bind _returnvalue_2 (Camera|GetCameraLocation _returnvalue))
  (Variables|Default|SetbCanFire false)
  (bind _result (Math|Integer|DecrementInt (Variables|Default|GetCurrentMagazine))
    (:%20%20
      (Default|CallOnAmmoChanged _result (Variables|Default|GetReserveAmmo))
      (bind (_outhit _returnvalue_3) (Collision|LineTraceByChannel _returnvalue_2 (+ (* (Math|Vector|GetForwardVector (Variables|/Script/Engine.PlayerCameraManager|GetTransformComponent _returnvalue)) (Variables|Default|GetMaxRange)) _returnvalue_2) "TraceTypeQuery1" false 0 "ForDuration"))
      (if _returnvalue_3
        (if (Utilities|DoesObjectImplementInterface (.hitactor _outhit) "/Game/Blueprints/BPI_Damageable.BPI_Damageable_C")
          (Class|BPIDamageable|ReceiveDamage(Message) (.hitactor _outhit) (Variables|Default|GetBaseDamage))))
      (Utilities|FlowControl|Delay (Variables|Default|GetFireRate))
      (Variables|Default|SetbCanFire true))))

(event Custom|TryReload
  (if (Math|Boolean|ANDBoolean (not (Variables|Default|GetbIsReloading)) (< (Variables|Default|GetCurrentMagazine) (Variables|Default|GetMaxMagazine)) (> (Variables|Default|GetReserveAmmo) 0))
    (CallFunction|Reload)))

(event Custom|Reload
  (Variables|Default|SetbIsReloading true)
  (Variables|Default|SetbCanFire false)
  (Utilities|FlowControl|Delay (Variables|Default|GetReloadSpeed))
  (Variables|Default|SetAmmoNeeded (- (Variables|Default|GetMaxMagazine) (Variables|Default|GetCurrentMagazine)))
  (if (>= (Variables|Default|GetReserveAmmo) (Variables|Default|GetAmmoNeeded))
    (Variables|Default|SetCurrentMagazine (+ (Variables|Default|GetCurrentMagazine) (Variables|Default|GetAmmoNeeded)))
    (Variables|Default|SetReserveAmmo (- (Variables|Default|GetReserveAmmo) (Variables|Default|GetAmmoNeeded)))
    (else
      (Variables|Default|SetCurrentMagazine (+ (Variables|Default|GetCurrentMagazine) (Variables|Default|GetReserveAmmo)))
      (Variables|Default|SetReserveAmmo 0)))
  (Default|CallOnAmmoChanged (Variables|Default|GetCurrentMagazine) (Variables|Default|GetReserveAmmo))
  (Variables|Default|SetbIsReloading false)
  (Variables|Default|SetbCanFire true))

(event EventBeginPlay
  (Variables|Default|SetbIsEquipped false)
  (bind _asbp_pbplayer_controller (Utilities|Casting|CastToBP_PBPlayerController (Game|GetPlayerController 0)))
  (Variables|Default|SetPCRef _asbp_pbplayer_controller))

(fn ConstructionScript)