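; Player character Blueprint with speed-scaled turn rate, crouch sliding, weapon aiming, damage handling and a grabbed state.
; Tick runs the slide check: holding crouch on ground slides on fast downhill movement or above walk speed on gentler ground, changing friction and adding slope-scaled force.
; A timeline blends camera arm length and FOV for aiming.
; Equipping and grab disabling swap Enhanced Input contexts; damage feeds the health component and updates the controller.
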(event Custom|CheckSliding
  (bind _returnvalue (Class|PBPlayerCharacter|GetMovementPtr))
  (bind _currentfloor (Variables|/Script/Engine.CharacterMovementComponent|GetCurrentFloor _returnvalue))
  (bind _velocity (Variables|/Script/Engine.MovementComponent|GetVelocity _returnvalue))
  (if (and (Variables|/Game/Characters/Player/PB/BP_PBPlayerController.BP_PBPlayerController_C|GetTryingToCrouch (Variables|Default|GetPCRef)) (not (AI|Components|NavMovement|IsFalling _returnvalue)))
    (bind _angle (CallFunction|GetSlopeAngle (.hitresult (Variables|/Script/Engine.CharacterMovementComponent|GetCurrentFloor _returnvalue))))
    (if (> _angle (Variables|Default|GetMinSlideAngle))
      (if (> (Math|Vector|DotProduct _velocity (CallFunction|GetDownSlopeDirection (.normal (.hitresult _currentfloor)))) (Variables|Default|GetMinSlopeSlideVelocity))
        (CallFunction|StartSliding :!label _label)
        (Physics|AddForce (Variables|Character|GetCharacterMovement) (/ (* (/ _angle 9e+01) (+ (* (CallFunction|GetDownSlopeDirection (.normal (.hitresult _currentfloor))) 1e+04) (.location (.hitresult _currentfloor)))) (Utilities|Time|GetWorldDeltaSeconds)))
        (else
          (CallFunction|StopSliding :!label _label_2)))
      (elif (> (Math|Vector|VectorLength _velocity) (Variables|/Script/PBCharacterMovement.PBPlayerMovement|GetWalkSpeed _returnvalue))
        (goto _label)
        (else
          (goto _label_2))))
    (else
      (goto _label_2))))

(event Custom|DisablePlayerInput
  (bind _pcref (Variables|Default|GetPCRef))
  (bind _returnvalue (PlayerController|LocalPlayerSubsystems|GetEnhancedInputLocalPlayerSubsystem _pcref))
  (Variables|Default|SetIsDisabled true)
  (Input|RemoveMappingContext _returnvalue "/Game/Input/IMC_GunEquipped.IMC_GunEquipped" "(bIgnoreAllPressedKeysUntilRelease=True,bForceImmediately=False,bNotifyUserSettings=False)")
  (Input|AddMappingContext _returnvalue "/Game/Input/IMC_Grabbed.IMC_Grabbed" 1 "(bIgnoreAllPressedKeysUntilRelease=True,bForceImmediately=False,bNotifyUserSettings=False)")
  (Pawn|Components|CharacterMovement|SetMovementMode (Variables|Character|GetCharacterMovement) "MOVE_None" 0))

(event Custom|EnablePlayerInput
  (bind _pcref (Variables|Default|GetPCRef))
  (bind _returnvalue (PlayerController|LocalPlayerSubsystems|GetEnhancedInputLocalPlayerSubsystem _pcref))
  (Variables|Default|SetIsDisabled false)
  (Input|RemoveMappingContext _returnvalue "/Game/Input/IMC_Grabbed.IMC_Grabbed" "(bIgnoreAllPressedKeysUntilRelease=True,bForceImmediately=False,bNotifyUserSettings=False)")
  (Input|AddMappingContext _returnvalue "/Game/Input/IMC_GunEquipped.IMC_GunEquipped" 0 "(bIgnoreAllPressedKeysUntilRelease=True,bForceImmediately=False,bNotifyUserSettings=False)")
  (Pawn|Components|CharacterMovement|SetMovementMode (Variables|Character|GetCharacterMovement) "MOVE_Walking" 0))

(event Custom|ResetMeshTransform
  (bind _mesh (Variables|Character|GetMesh))
  (Transformation|SetRelativeLocation _mesh "0.000000,0.000000,-90.000000" false false)
  (Transformation|SetRelativeRotation _mesh "0.000000,-90.000000,0.000000" false false))

(event Custom|DefaultMeshTransform
  (bind _mesh (Variables|Character|GetMesh))
  (Transformation|SetRelativeLocation _mesh "0, 0, 0" false false)
  (Transformation|SetRelativeRotation _mesh "0, 0, 0" false false))

(event Custom|OnAimStart
  (bind _aimalpha (Timeline|AimTimeline Play)
    (:Update
      (Variables|/Script/Engine.SpringArmComponent|SetTargetArmLength (Variables|Components|GetSpringArm) (Math|Float|Lerp (Variables|Default|GetAimSpringArmStartLength) (Variables|Default|GetAimSpringArmEndLength) _aimalpha))
      (Camera|SetFieldOfView (Variables|Components|GetCamera) (Math|Float|Lerp (Variables|Default|GetAimStartFOV) (Variables|Default|GetAimEndFOV) _aimalpha)))))

(event Custom|OnAimEnd
  (bind _aimalpha (Timeline|AimTimeline Reverse)
    (:Update
      (Variables|/Script/Engine.SpringArmComponent|SetTargetArmLength (Variables|Components|GetSpringArm) (Math|Float|Lerp (Variables|Default|GetAimSpringArmStartLength) (Variables|Default|GetAimSpringArmEndLength) _aimalpha))
      (Camera|SetFieldOfView (Variables|Components|GetCamera) (Math|Float|Lerp (Variables|Default|GetAimStartFOV) (Variables|Default|GetAimEndFOV) _aimalpha)))))

(event Custom|OnWeaponUnequipped
  (Variables|Default|SetEquippedWeapon 0)
  (Variables|Default|SetbIsAiming false))

(event EventBeginPlay
  (bind _asbp_pbplayer_controller (Utilities|Casting|CastToBP_PBPlayerController (Game|GetPlayerController 0)))
  (Variables|Default|SetPCRef _asbp_pbplayer_controller)
  (Variables|Default|SetAimSpringArmStartLength (Variables|/Script/Engine.SpringArmComponent|GetTargetArmLength (Variables|Components|GetSpringArm)))
  (Variables|Default|SetAimStartFOV (Variables|/Script/Engine.CameraComponent|GetFieldOfView (Variables|Components|GetCamera)))
  (Variables|Default|SetAimSpringArmEndLength (* (Variables|Default|GetAimSpringArmStartLength) (Variables|Default|GetAimSpringArmLengthMultiplier)))
  (Variables|Default|SetAimEndFOV (* (Variables|Default|GetAimStartFOV) (Variables|Default|GetAimFOVMultiplier)))
  (Variables|Default|SetDeltaTurnRate (Math|Rotator|MakeRotator 0.0 0.0 (- (.Yaw (Math|Rotator|BreakRotator (Variables|Default|GetMaxTurnRate))) (.Yaw (Math|Rotator|BreakRotator (Variables|Default|GetMinTurnRate)))))))

(event EventDamage
  (params (DamageAmount :type Float%20%28double-precision%29))
  (bind _bp_healthcomponent (Variables|Default|GetBP_HealthComponent))
  (Default|TakeDamage _bp_healthcomponent DamageAmount)
  (if (not (Variables|/Game/Gameplay/Components/BP_HealthComponent.BP_HealthComponent_C|GetbIsDead _bp_healthcomponent))
    (Default|UpdateHealth (Variables|Default|GetPCRef) (Variables|/Game/Gameplay/Components/BP_HealthComponent.BP_HealthComponent_C|GetCurrentHealth _bp_healthcomponent))))

(event EventOnWeaponEquipped
  (params (EquippedWeapon :type BP%20Weapon%20Base%20Object%20Reference))
  (bind _pcref (Variables|Default|GetPCRef))
  (bind _returnvalue (PlayerController|LocalPlayerSubsystems|GetEnhancedInputLocalPlayerSubsystem _pcref))
  (Input|RemoveMappingContext _returnvalue "/Game/Input/IMC_Unarmed.IMC_Unarmed" "(bIgnoreAllPressedKeysUntilRelease=True,bForceImmediately=False,bNotifyUserSettings=False)")
  (Input|AddMappingContext _returnvalue "/Game/Input/IMC_GunEquipped.IMC_GunEquipped" 0 "(bIgnoreAllPressedKeysUntilRelease=True,bForceImmediately=False,bNotifyUserSettings=False)")
  (bind _output_get (Variables|Default|SetEquippedWeapon EquippedWeapon))
  (EventDispatchers|BindEventtoOnAmmoChanged _output_get (EventDispatchers|CreateEvent (Variables|Default|GetPCRef) :!event UpdateAmmo))
  (Default|CallOnAmmoChanged _output_get (Variables|/Game/Gameplay/Weapons/Base/BP_Weapon_Base.BP_Weapon_Base_C|GetCurrentMagazine _output_get) (Variables|/Game/Gameplay/Weapons/Base/BP_Weapon_Base.BP_Weapon_Base_C|GetReserveAmmo _output_get)))

(event EventOnLanded
  (params (Hit :type Hit%20Result%20Structure%20%28by%20ref%29))
  (Animation|PlayAnimMontage "/Game/Characters/Mannequins/Anims/Unarmed/Jump/AM_Land.AM_Land" 1.0 "None"))

(event EventTick
  (params (DeltaSeconds :type Float%20%28single-precision%29))
  (bind _returnvalue (Class|PBPlayerCharacter|GetMovementPtr))
  (bind _returnvalue_2 (Class|PBPlayerCharacter|GetMovementPtr))
  (bind _output_get (Variables|Default|SetCurrentSpeedPercent (/ (Math|Vector|VectorLength (Transformation|GetVelocity)) (Variables|/Script/PBCharacterMovement.PBPlayerMovement|GetSprintSpeed _returnvalue))))
  (Variables|/Script/Engine.CharacterMovementComponent|SetRotationRate _returnvalue (Math|Rotator|MakeRotator 0.0 0.0 (Math|Float|Clamp(Float) (+ (.Yaw (Math|Rotator|BreakRotator (Variables|Default|GetMinTurnRate))) (* _output_get (.Yaw (Math|Rotator|BreakRotator (Variables|Default|GetDeltaTurnRate))))) 0.0 (.Yaw (Math|Rotator|BreakRotator (Variables|Default|GetMaxTurnRate))))))
  (if (and (Variables|/Game/Characters/Player/PB/BP_PBPlayerController.BP_PBPlayerController_C|GetTryingToCrouch (Variables|Default|GetPCRef)) (AI|Components|NavMovement|IsFalling (Class|PBPlayerCharacter|GetMovementPtr)))
    (Variables|/Script/PBCharacterMovement.PBPlayerMovement|SetCrouchTime _returnvalue_2 0.0)
    (elif (and (not (AI|Components|NavMovement|IsFalling (Class|PBPlayerCharacter|GetMovementPtr))) (not (Variables|/Game/Characters/Player/PB/BP_PBPlayerController.BP_PBPlayerController_C|GetTryingToCrouch (Variables|Default|GetPCRef))))
      (Variables|/Script/PBCharacterMovement.PBPlayerMovement|SetCrouchTime _returnvalue_2 0.4)))
  (CallFunction|CheckSliding))

(fn ConstructionScript)

(fn GetSlopeAngle
  (params (FloorHit :type Hit%20Result%20Structure))
  (return (Class|KismetMathLibrary|DegAcos (Math|Vector|DotProduct (.normal FloorHit) (Math|Vector|VectorUp)))))

(fn GetDownSlopeDirection
  (params (FloorNormal :type Vector))
  (return (Math|Vector|NegateVector (Math|Vector|Normalize (Math|Vector|CrossProduct (Math|Vector|CrossProduct FloorNormal (Math|Vector|VectorUp)) FloorNormal)))))

(fn StopSliding
  (bind _returnvalue (Class|PBPlayerCharacter|GetMovementPtr))
  (Variables|Default|SetIsSliding false)
  (Variables|/Script/Engine.CharacterMovementComponent|SetGroundFriction _returnvalue (Variables|Default|GetNormalFriction))
  (Variables|/Script/PBCharacterMovement.PBPlayerMovement|SetGroundAccelerationMultiplier _returnvalue 5.0))

(fn StartSliding
  (bind _returnvalue (Class|PBPlayerCharacter|GetMovementPtr))
  (Variables|Default|SetIsSliding true)
  (Variables|/Script/Engine.CharacterMovementComponent|SetGroundFriction _returnvalue (Variables|Default|GetSlideFriction))
  (Variables|/Script/PBCharacterMovement.PBPlayerMovement|SetGroundAccelerationMultiplier _returnvalue 1e+01))

(fn GetSliding
  (return (Variables|Default|GetIsSliding)))