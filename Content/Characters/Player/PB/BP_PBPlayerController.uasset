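; Player controller for BP_PBPlayerCharacter that turns Enhanced Input into movement, sprint, crouch, jump, aim and weapon actions.
; It creates WBP_HUD with health and ammo updates, and broadcasts mash input.
; Movement is camera-yaw relative, backpedalling rescales run speed and acceleration, and Tick cancels sprint without forward or strafe input or when moving backward.
; While sliding, move input instead steers horizontal velocity toward a camera-based direction, preserving speed.
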(event Custom|CreateHUD
  (bind _returnvalue (UserInterface|CreateWidget "/Game/UI/HUD/WBP_HUD.WBP_HUD_C"))
  (bind _output_get (Variables|Default|SetHUD _returnvalue))
  (UserInterface|Viewport|AddtoPlayerScreen _output_get))

(event Custom|UpdateHealth
  (params (NewHealth :type Float%20%28double-precision%29))
  (Progress|SetPercent (Variables|/Game/UI/HUD/WBP_HUD.WBP_HUD_C|GetHealthBar (Variables|Default|GetHUD)) (/ NewHealth 1e+02)))

(event Custom|UpdateAmmo
  (params (CurrentMagazine :type Integer) (ReserveAmmo :type Integer))
  (Rendering|Components|TextRender|SetText (Variables|/Game/UI/HUD/WBP_HUD.WBP_HUD_C|GetCurrentMagazineText (Variables|Default|GetHUD)) (Utilities|Text|FormatText "{CurrentMagazine}/{ReserveAmmo}" CurrentMagazine ReserveAmmo)))

(event Input|EnhancedActionEvents|EnhancedInputActionIA_PrimaryFire
  (params (ActionValue :type Boolean) (ElapsedSeconds :type Float%20%28double-precision%29) (TriggeredSeconds :type Float%20%28double-precision%29) (InputAction :type Input%20Action%20Object%20Reference :default "/Game/Input/Actions/IA_PrimaryFire.IA_PrimaryFire"))
  (bind _controlledcharacterref (Variables|Default|GetControlledCharacterRef))
  (bind _equippedweapon (Variables|/Game/Characters/Player/PB/BP_PBPlayerCharacter.BP_PBPlayerCharacter_C|GetEquippedWeapon _controlledcharacterref))
  (if (and (Utilities|IsValid _equippedweapon) (Variables|/Game/Characters/Player/PB/BP_PBPlayerCharacter.BP_PBPlayerCharacter_C|GetbIsAiming _controlledcharacterref))
    (Default|TryFire _equippedweapon)))

(event Input|EnhancedActionEvents|EnhancedInputActionIA_Reload
  (params (ActionValue :type Boolean) (ElapsedSeconds :type Float%20%28double-precision%29) (TriggeredSeconds :type Float%20%28double-precision%29) (InputAction :type Input%20Action%20Object%20Reference :default "/Game/Input/Actions/IA_Reload.IA_Reload"))
  (bind _controlledcharacterref (Variables|Default|GetControlledCharacterRef))
  (bind _equippedweapon (Variables|/Game/Characters/Player/PB/BP_PBPlayerCharacter.BP_PBPlayerCharacter_C|GetEquippedWeapon _controlledcharacterref))
  (if (Utilities|IsValid _equippedweapon)
    (Default|TryReload _equippedweapon)))

(event Input|EnhancedActionEvents|EnhancedInputActionIA_Jump
  (params (ActionValue :type Boolean) (ElapsedSeconds :type Float%20%28double-precision%29) (TriggeredSeconds :type Float%20%28double-precision%29) (InputAction :type Input%20Action%20Object%20Reference :default "/Game/Input/Actions/IA_Jump.IA_Jump"))
  (bind _controlledcharacterref (Variables|Default|GetControlledCharacterRef))
  (:Triggered
    (Character|Jump _controlledcharacterref))
  (:Completed
    (Character|StopJumping _controlledcharacterref)))

(event Input|EnhancedActionEvents|EnhancedInputActionIA_Crouch
  (params (ActionValue :type Boolean) (ElapsedSeconds :type Float%20%28double-precision%29) (TriggeredSeconds :type Float%20%28double-precision%29) (InputAction :type Input%20Action%20Object%20Reference :default "/Game/Input/Actions/IA_Crouch.IA_Crouch"))
  (bind _controlledcharacterref (Variables|Default|GetControlledCharacterRef))
  (:Triggered
    (Character|Crouch _controlledcharacterref))
  (:Completed
    (Character|UnCrouch _controlledcharacterref)))

(event Input|EnhancedActionEvents|EnhancedInputActionIA_Mash
  (params (ActionValue :type Boolean) (ElapsedSeconds :type Float%20%28double-precision%29) (TriggeredSeconds :type Float%20%28double-precision%29) (InputAction :type Input%20Action%20Object%20Reference :default "/Game/Input/Actions/IA_Mash.IA_Mash"))
  (Default|CallOnPlayerMashInput))

(event Input|EnhancedActionEvents|EnhancedInputActionIA_Aim
  (params (ActionValue :type Boolean) (ElapsedSeconds :type Float%20%28double-precision%29) (TriggeredSeconds :type Float%20%28double-precision%29) (InputAction :type Input%20Action%20Object%20Reference :default "/Game/Input/Actions/IA_Aim.IA_Aim"))
  (bind _controlledcharacterref (Variables|Default|GetControlledCharacterRef))
  (:Started
    (if (Utilities|IsValid (Variables|/Game/Characters/Player/PB/BP_PBPlayerCharacter.BP_PBPlayerCharacter_C|GetEquippedWeapon _controlledcharacterref))
      (Variables|/Game/Characters/Player/PB/BP_PBPlayerCharacter.BP_PBPlayerCharacter_C|SetbIsAiming _controlledcharacterref true)
      (Default|OnAimStart _controlledcharacterref)))
  (:Canceled
    (Variables|/Game/Characters/Player/PB/BP_PBPlayerCharacter.BP_PBPlayerCharacter_C|SetbIsAiming _controlledcharacterref false :!label _label)
    (Default|OnAimEnd _controlledcharacterref))
  (:Completed
    (goto _label)))

(event Input|EnhancedActionEvents|EnhancedInputActionIA_Sprint
  (params (ActionValue :type Boolean) (ElapsedSeconds :type Float%20%28double-precision%29) (TriggeredSeconds :type Float%20%28double-precision%29) (InputAction :type Input%20Action%20Object%20Reference :default "/Game/Input/Actions/IA_Sprint.IA_Sprint"))
  (bind _controlledcharacterref (Variables|Default|GetControlledCharacterRef))
  (:Started
    (Class|PBPlayerCharacter|SetSprinting _controlledcharacterref (not (Class|PBPlayerCharacter|IsSprinting _controlledcharacterref)))))

(event Input|EnhancedActionEvents|EnhancedInputActionIA_MoveForward
  (params (ActionValue :type Float%20%28double-precision%29) (ElapsedSeconds :type Float%20%28double-precision%29) (TriggeredSeconds :type Float%20%28double-precision%29) (InputAction :type Input%20Action%20Object%20Reference :default "/Game/Input/Actions/IA_MoveForward.IA_MoveForward"))
  (bind _controlledcharacterref (Variables|Default|GetControlledCharacterRef))
  (bind _returnvalue (Class|PBPlayerCharacter|GetMovementPtr _controlledcharacterref))
  (bind _backwardspeedmultiplier (Variables|/Game/Characters/Player/PB/BP_PBPlayerCharacter.BP_PBPlayerCharacter_C|GetBackwardSpeedMultiplier _controlledcharacterref))
  (if (< ActionValue 0.0)
    (Variables|/Script/PBCharacterMovement.PBPlayerMovement|SetRunSpeed _returnvalue (* (Variables|Default|GetOriginalRunSpeed) _backwardspeedmultiplier))
    (Variables|/Script/PBCharacterMovement.PBPlayerMovement|SetGroundAccelerationMultiplier _returnvalue (/ (Variables|Default|GetOriginalGroundAccelerationMultiplier) _backwardspeedmultiplier))
    (else
      (Variables|/Script/PBCharacterMovement.PBPlayerMovement|SetRunSpeed _returnvalue (Variables|Default|GetOriginalRunSpeed))
      (Variables|/Script/PBCharacterMovement.PBPlayerMovement|SetGroundAccelerationMultiplier _returnvalue (Variables|Default|GetOriginalGroundAccelerationMultiplier))))
  (if (Default|GetSliding _controlledcharacterref)
    (CallFunction|SteerSlidingVelocity (Variables|Default|GetControlledCharacterRef) (Game|GetPlayerCameraManager 0) (stale Input|EnhancedActionEvents|EnhancedInputActionIA_MoveRight ActionValue) ActionValue)
    (else
      (Pawn|Input|AddMovementInput (Pawn|GetControlledPawn) (Math|Vector|GetForwardVector (Math|Rotator|MakeRotator 0.0 0.0 (.Yaw (Math|Rotator|BreakRotator (Camera|GetCameraRotation (Game|GetPlayerCameraManager 0)))))) ActionValue false))))

(event Input|EnhancedActionEvents|EnhancedInputActionIA_MoveRight
  (params (ActionValue :type Float%20%28double-precision%29) (ElapsedSeconds :type Float%20%28double-precision%29) (TriggeredSeconds :type Float%20%28double-precision%29) (InputAction :type Input%20Action%20Object%20Reference :default "/Game/Input/Actions/IA_MoveRight.IA_MoveRight"))
  (if (Default|GetSliding (Variables|Default|GetControlledCharacterRef))
    (CallFunction|SteerSlidingVelocity (Variables|Default|GetControlledCharacterRef) (Game|GetPlayerCameraManager 0) ActionValue (stale Input|EnhancedActionEvents|EnhancedInputActionIA_MoveForward ActionValue))
    (else
      (Pawn|Input|AddMovementInput (Pawn|GetControlledPawn) (Math|Vector|GetRightVector (Math|Rotator|MakeRotator 0.0 0.0 (.Yaw (Math|Rotator|BreakRotator (Camera|GetCameraRotation (Game|GetPlayerCameraManager 0)))))) ActionValue false))))

(event Input|EnhancedActionEvents|EnhancedInputActionIA_Turn
  (params (ActionValue :type Float%20%28double-precision%29) (ElapsedSeconds :type Float%20%28double-precision%29) (TriggeredSeconds :type Float%20%28double-precision%29) (InputAction :type Input%20Action%20Object%20Reference :default "/Game/Input/Actions/IA_Turn.IA_Turn"))
  (Pawn|Input|AddControllerYawInput (Pawn|GetControlledPawn) ActionValue))

(event Input|EnhancedActionEvents|EnhancedInputActionIA_LookUp
  (params (ActionValue :type Float%20%28double-precision%29) (ElapsedSeconds :type Float%20%28double-precision%29) (TriggeredSeconds :type Float%20%28double-precision%29) (InputAction :type Input%20Action%20Object%20Reference :default "/Game/Input/Actions/IA_LookUp.IA_LookUp"))
  (Pawn|Input|AddControllerPitchInput (Pawn|GetControlledPawn) ActionValue))

(event EventPossess
  (params (PossessedPawn :type Pawn%20Object%20Reference))
  (bind _asbp_pbplayer_character (Utilities|Casting|CastToBP_PBPlayerCharacter PossessedPawn))
  (bind _output_get (Variables|Default|SetControlledCharacterRef _asbp_pbplayer_character))
  (Variables|Default|SetOriginalRunSpeed (Variables|/Script/PBCharacterMovement.PBPlayerMovement|GetRunSpeed (Class|PBPlayerCharacter|GetMovementPtr _output_get)))
  (Variables|Default|SetOriginalGroundAccelerationMultiplier (Variables|/Script/PBCharacterMovement.PBPlayerMovement|GetGroundAccelerationMultiplier (Class|PBPlayerCharacter|GetMovementPtr _output_get))))

(event EventTick
  (params (DeltaSeconds :type Float%20%28single-precision%29))
  (bind _returnvalue (Input|EnhancedActionValues|GetIA_MoveForward))
  (if (or (< _returnvalue 0.0) (and (== _returnvalue 0.0) (== (Input|EnhancedActionValues|GetIA_MoveRight) 0.0)))
    (Class|PBPlayerCharacter|SetSprinting (Variables|Default|GetControlledCharacterRef) false)))

(event EventBeginPlay
  (Input|AddMappingContext (PlayerController|LocalPlayerSubsystems|GetEnhancedInputLocalPlayerSubsystem) "/Game/Input/IMC_Unarmed.IMC_Unarmed" 0 "(bIgnoreAllPressedKeysUntilRelease=True,bForceImmediately=False,bNotifyUserSettings=False)")
  (CallFunction|CreateHUD))

(fn ConstructionScript)

(fn SteerSlidingVelocity
  (params (ControlledCharacterRef :type BP%20PB%20Player%20Character%20Object%20Reference) (PlayerCameraManager :type Player%20Camera%20Manager%20Object%20Reference) (InputX :type Float%20%28double-precision%29) (InputY :type Float%20%28double-precision%29))
  (bind _returnvalue (Class|PBPlayerCharacter|GetMovementPtr ControlledCharacterRef))
  (bind _returnvalue_2 (Camera|GetCameraRotation PlayerCameraManager))
  (bind _output_get (LocalVariables|SetCurrentVelocity (Variables|/Script/Engine.MovementComponent|GetVelocity _returnvalue)))
  (bind _output_get_2 (LocalVariables|SetHorizontalVelocity (Math|Vector|MakeVector (.X (Math|Vector|BreakVector _output_get)) (.Y (Math|Vector|BreakVector _output_get)) 0.0)))
  (bind _output_get_3 (LocalVariables|SetCurrentSpeed (Math|Vector|VectorLength _output_get_2)))
  (bind _output_get_4 (LocalVariables|SetCurrentDirection (Math|Vector|Normalize _output_get_2)))
  (bind _output_get_5 (LocalVariables|SetDesiredDirection (Math|Vector|Normalize (+ (* InputX (Math|Vector|GetRightVector _returnvalue_2)) (* InputY (Math|Vector|GetForwardVector _returnvalue_2))))))
  (bind _output_get_6 (LocalVariables|SetNewDirection (Math|Vector2D|Normalize2D (Class|KismetMathLibrary|Vector2DInterptoConstant (Math|Conversions|ToVector2D(Vector) _output_get_4) (Math|Conversions|ToVector2D(Vector) _output_get_5) (Utilities|Time|GetWorldDeltaSeconds) (* (Variables|Default|GetSlideControl) 1e+01)))))
  (bind _output_get_7 (LocalVariables|SetNewHorizontalVelocity (* _output_get_6 _output_get_3)))
  (bind _output_get_8 (LocalVariables|SetFinalVelocity (Math|Vector|MakeVector (.X (Math|Vector2D|BreakVector2D _output_get_7)) (.Y (Math|Vector2D|BreakVector2D _output_get_7)) (.Z (Math|Vector|BreakVector _output_get)))))
  (Variables|/Script/Engine.MovementComponent|SetVelocity _returnvalue _output_get_8))