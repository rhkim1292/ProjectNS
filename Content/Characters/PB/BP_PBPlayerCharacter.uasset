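; Player character Blueprint that adds crouch sliding and handles weapon ammo events, damage and control toggling.
; A looping timer polls floor slope and velocity while crouched, sliding on fast downhill movement or above walk speed on flatter ground.
; Sliding swaps ground friction and adds a slope-scaled force, built from downslope direction plus floor hit location.
; Equipping binds and fires ammo-changed; damage feeds the health component, updating the controller's health while alive.
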(event Custom|CheckSliding
  (bind _returnvalue (Class|PBPlayerCharacter|GetMovementPtr))
  (bind _currentfloor (Variables|/Script/Engine.CharacterMovementComponent|GetCurrentFloor _returnvalue))
  (bind _velocity (Variables|/Script/Engine.MovementComponent|GetVelocity _returnvalue))
  (bind _direction (CallFunction|GetDownSlopeDirection (.normal (.hitresult _currentfloor))))
  (if (AI|Components|NavMovement|IsCrouching _returnvalue)
    (bind _angle (CallFunction|GetSlopeAngle (.hitresult (Variables|/Script/Engine.CharacterMovementComponent|GetCurrentFloor _returnvalue))))
    (if (> _angle (Variables|Default|GetMinSlideAngle))
      (if (> (Math|Vector|DotProduct _velocity _direction) (Variables|Default|GetMinSlopeSlideVelocity))
        (CallFunction|StartSliding :!label _label)
        (Physics|AddForce (Variables|Character|GetCharacterMovement) (* (/ _angle 9e+01) (+ (* _direction 2e+06) (.location (.hitresult _currentfloor)))))
        (else
          (CallFunction|StopSliding :!label _label_2)))
      (elif (> (Math|Vector|DotProduct (Math|Vector|Normalize _velocity) _velocity) (Variables|/Script/PBCharacterMovement.PBPlayerMovement|GetWalkSpeed _returnvalue))
        (goto _label)
        (else
          (goto _label_2))))
    (else
      (goto _label_2))))

(event Custom|DisablePlayerControl
  (Input|DisableInput (Variables|Default|GetPCRef))
  (Pawn|Components|CharacterMovement|SetMovementMode (Variables|Character|GetCharacterMovement) "MOVE_None" 0))

(event Custom|ReEnablePlayerControl
  (Input|EnableInput (Variables|Default|GetPCRef))
  (Pawn|Components|CharacterMovement|SetMovementMode (Variables|Character|GetCharacterMovement) "MOVE_Walking" 0))

(event EventBeginPlay
  ;[0.15 0.15 0.15 0.5] Polling for slopes
  (Utilities|Time|SetTimerbyFunctionName 0 "CheckSliding" 0.1 true)
  (bind _asbp_pbplayer_controller (Utilities|Casting|CastToBP_PBPlayerController (Game|GetPlayerController 0)))
  (Variables|Default|SetPCRef _asbp_pbplayer_controller))

(event EventDamage
  (params (DamageAmount :type Float%20%28double-precision%29))
  (bind _bp_healthcomponent (Variables|Default|GetBP_HealthComponent))
  (Default|TakeDamage _bp_healthcomponent DamageAmount)
  (if (not (Variables|/Game/Gameplay/Components/BP_HealthComponent.BP_HealthComponent_C|GetbIsDead _bp_healthcomponent))
    (Default|UpdateHealth (Variables|Default|GetPCRef) (Variables|/Game/Gameplay/Components/BP_HealthComponent.BP_HealthComponent_C|GetCurrentHealth _bp_healthcomponent))))

(event EventOnWeaponEquipped
  (params (EquippedWeapon :type BP%20Weapon%20Base%20Object%20Reference))
  (bind _output_get (Variables|Default|SetEquippedWeapon EquippedWeapon))
  (EventDispatchers|BindEventtoOnAmmoChanged _output_get (EventDispatchers|CreateEvent (Variables|Default|GetPCRef) :!event UpdateAmmo))
  (Default|CallOnAmmoChanged _output_get (Variables|/Game/Gameplay/Weapons/Base/BP_Weapon_Base.BP_Weapon_Base_C|GetCurrentMagazine _output_get) (Variables|/Game/Gameplay/Weapons/Base/BP_Weapon_Base.BP_Weapon_Base_C|GetReserveAmmo _output_get)))

(fn ConstructionScript)

(fn GetSlopeAngle
  (params (FloorHit :type Hit%20Result%20Structure))
  (return (Class|KismetMathLibrary|DegAcos (Math|Vector|DotProduct (.normal FloorHit) (Math|Vector|VectorUp)))))

(fn GetDownSlopeDirection
  (params (FloorNormal :type Vector))
  (return (Math|Vector|NegateVector (Math|Vector|Normalize (Math|Vector|CrossProduct (Math|Vector|CrossProduct FloorNormal (Math|Vector|VectorUp)) FloorNormal)))))

(fn StopSliding
  (Variables|Default|SetIsSliding false)
  (Variables|/Script/Engine.CharacterMovementComponent|SetGroundFriction (Class|PBPlayerCharacter|GetMovementPtr) (Variables|Default|GetNormalFriction)))

(fn StartSliding
  (Variables|Default|SetIsSliding true)
  (Variables|/Script/Engine.CharacterMovementComponent|SetGroundFriction (Class|PBPlayerCharacter|GetMovementPtr) (Variables|Default|GetSlideFriction)))

(fn GetSliding
  (return (Variables|Default|GetIsSliding)))