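; Zombie enemy that grabs the player when its lunge hitbox overlaps them, and forwards incoming damage to its health component.
; A grab stops zombie movement, disables player control and attaches the player to a socket.
; Function-name timers deal repeated damage, then detach the player after a fixed hold.
; Nothing here starts the lunge, and ending the grab does not restore movement, control, hitbox collision or the grabbing flag.
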(event OnComponentBeginOverlap(LungeHitbox)
  (params (OverlappedComponent :type Primitive%20Component%20Object%20Reference) (OtherActor :type Actor%20Object%20Reference) (OtherComp :type Primitive%20Component%20Object%20Reference) (OtherBodyIndex :type Integer) (bFromSweep :type Boolean) (SweepResult :type Hit%20Result%20Structure%20%28by%20ref%29))
  (if (and (Variables|Default|GetbIsLunging) (not (Variables|Default|GetbIsGrabbing)))
    (bind _asbp_pbplayer_character (Utilities|Casting|CastToBP_PBPlayerCharacter OtherActor))
    (CallFunction|InitiateGrab _asbp_pbplayer_character)))

(event Custom|InitiateGrab
  (params (GrabbedPlayer :type BP%20PB%20Player%20Character%20Object%20Reference))
  (Development|PrintString "Grab Initiated")
  (Variables|Default|SetbIsGrabbing true)
  (Variables|Default|SetbIsLunging false)
  (Collision|SetCollisionEnabled (Variables|Default|GetLungeHitbox) "NoCollision")
  (Pawn|Components|CharacterMovement|SetMovementMode (Variables|Character|GetCharacterMovement) "MOVE_None" 0)
  (Default|DisablePlayerControl GrabbedPlayer)
  (Transformation|AttachActorToActor GrabbedPlayer self "GrabSocket" "KeepRelative" "KeepRelative" "KeepRelative" true)
  (Utilities|Time|SetTimerbyFunctionName 0 "ApplyGrabDamage" 0.5 true)
  (Utilities|Time|SetTimerbyFunctionName 0 "EndGrab" 3.0))

(event Custom|ApplyGrabDamage
  (bind _grabbedplayer (Variables|Default|GetGrabbedPlayer))
  (if (Utilities|IsValid _grabbedplayer)
    (Default|ReceiveDamage _grabbedplayer 15.0)))

(event Custom|EndGrab
  (Development|PrintString "Grab Ended")
  (Utilities|Time|ClearTimerbyFunctionName 0 "ApplyGrabDamage")
  (Transformation|DetachFromActor (Variables|Default|GetGrabbedPlayer) "KeepRelative" "KeepRelative" "KeepRelative"))

(event EventBeginPlay
  (Components|Sphere|SetSphereRadius (Variables|Default|GetLungeHitbox) (Variables|Default|GetLungeHitboxRadius) true))

(event EventDamage
  (params (DamageAmount :type Float%20%28double-precision%29))
  (Default|TakeDamage (Variables|Default|GetBP_HealthComponent) DamageAmount))

(fn ConstructionScript)