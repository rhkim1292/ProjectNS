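; AI controller for the zombie enemy that runs the BT_Zombie behavior tree.
; On possess, it copies its tuning variables for wandering, idling, chasing, lunging and grabbing into the blackboard.
; AI Perception updates set the player-in-sight flag and store the sensed actor's location, without checking that it is the player.
; A failed sense clears only the flag, leaving the last known location in place.
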(event OnTargetPerceptionUpdated(AIPerception)
  (params (Actor :type Actor%20Object%20Reference) (Stimulus :type AI%20Stimulus%20Structure))
  (bind _returnvalue (AI|GetBlackboard 0))
  (if (.bsuccessfullysensed Stimulus)
    (AI|Components|Blackboard|SetValueasBool _returnvalue (Variables|Default|GetPlayerInSightKeyName) true)
    (AI|Components|Blackboard|SetValueasVector _returnvalue (Variables|Default|GetPlayerLocationKeyName) (Transformation|GetActorLocation Actor))
    (else
      (AI|Components|Blackboard|SetValueasBool _returnvalue (Variables|Default|GetPlayerInSightKeyName) false))))

(event EventPossess
  (params (PossessedPawn :type Pawn%20Object%20Reference))
  (bind _returnvalue (AI|GetBlackboard 0))
  (AI|RunBehaviorTree "/Game/AI/BehaviorTrees/BT_Zombie.BT_Zombie")
  (AI|Components|Blackboard|SetValueasFloat _returnvalue (Variables|Default|GetLungeRangeKeyName) (Variables|Default|GetLungeRange))
  (AI|Components|Blackboard|SetValueasFloat _returnvalue (Variables|Default|GetWanderRadiusKeyName) (Variables|Default|GetWanderRadius))
  (AI|Components|Blackboard|SetValueasFloat _returnvalue (Variables|Default|GetChaseSpeedKeyName) (Variables|Default|GetChaseSpeed))
  (AI|Components|Blackboard|SetValueasFloat _returnvalue (Variables|Default|GetWanderSpeedKeyName) (Variables|Default|GetWanderSpeed))
  (AI|Components|Blackboard|SetValueasFloat _returnvalue (Variables|Default|GetLungeSpeedKeyName) (Variables|Default|GetLungeSpeed))
  (AI|Components|Blackboard|SetValueasFloat _returnvalue (Variables|Default|GetLungeTurnSpeedKeyName) (Variables|Default|GetLungeTurnSpeed))
  (AI|Components|Blackboard|SetValueasFloat _returnvalue (Variables|Default|GetWanderTurnSpeedKeyName) (Variables|Default|GetWanderTurnSpeed))
  (AI|Components|Blackboard|SetValueasFloat _returnvalue (Variables|Default|GetMinIdleTimeKeyName) (Variables|Default|GetMinIdleTime))
  (AI|Components|Blackboard|SetValueasFloat _returnvalue (Variables|Default|GetMaxIdleTimeKeyName) (Variables|Default|GetMaxIdleTime))
  (AI|Components|Blackboard|SetValueasFloat _returnvalue (Variables|Default|GetLungeDurationKeyName) (Variables|Default|GetLungeDuration))
  (AI|Components|Blackboard|SetValueasFloat _returnvalue (Utilities|Name|MakeLiteralName "GrabDuration") (Variables|Default|GetGrabDuration))
  (AI|Components|Blackboard|SetValueasFloat _returnvalue (Utilities|Name|MakeLiteralName "GrabDamagePerSecond") (Variables|Default|GetGrabDamagePerSecond))
  (AI|Components|Blackboard|SetValueasFloat _returnvalue (Utilities|Name|MakeLiteralName "LungeCooldownDuration") (Variables|Default|GetLungeCooldownDuration)))

(fn ConstructionScript)