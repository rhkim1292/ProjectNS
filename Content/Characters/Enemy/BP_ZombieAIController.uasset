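; AI controller for the zombie enemy that links its perception to behavior tree decisions.
; On possessing a BP_ZombieEnemy, it runs BT_Zombie, copies the pawn's lunge range into the blackboard and prints it for debugging.
; Perception updates set the player-in-sight flag and location for any sensed actor, without filtering.
; Losing the stimulus clears only the flag, leaving the last known location in the blackboard.
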(event OnTargetPerceptionUpdated(AIPerception)
  (params (Actor :type Actor%20Object%20Reference) (Stimulus :type AI%20Stimulus%20Structure))
  (bind _returnvalue (AI|GetBlackboard 0))
  (if (.bsuccessfullysensed Stimulus)
    (AI|Components|Blackboard|SetValueasBool _returnvalue (Variables|Default|GetPlayerInSightKeyName) true)
    (AI|Components|Blackboard|SetValueasVector _returnvalue (Variables|Default|GetPlayerLocationKeyName) (Transformation|GetActorLocation Actor))
    (else
      (AI|Components|Blackboard|ClearValue _returnvalue (Variables|Default|GetPlayerInSightKeyName)))))

(event EventPossess
  (params (PossessedPawn :type Pawn%20Object%20Reference))
  (bind _returnvalue (AI|GetBlackboard 0))
  (bind _lungerangekeyname (Variables|Default|GetLungeRangeKeyName))
  (bind _asbp_zombie_enemy (Utilities|Casting|CastToBP_ZombieEnemy PossessedPawn))
  (AI|RunBehaviorTree "/Game/BehaviorTrees/BT_Zombie.BT_Zombie")
  (AI|Components|Blackboard|SetValueasFloat _returnvalue _lungerangekeyname (Variables|/Game/Characters/Enemy/BP_ZombieEnemy.BP_ZombieEnemy_C|GetLungeRange _asbp_zombie_enemy))
  (Development|PrintString (Utilities|String|Append "LungeRange BB Value: " (Utilities|String|ToString(Float) (Class|BlackboardComponent|GetValueasFloat _returnvalue _lungerangekeyname)))))

(fn ConstructionScript)