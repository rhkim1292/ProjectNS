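; Zombie enemy character that lunges at the player and grabs on contact, with incoming damage forwarded to its health component.
; During a lunge it speeds up, steering toward the player each tick through interpolated rotation, and enables a sphere hitbox.
; An overlap stops movement, disables player control, attaches the player to a socket and starts timed repeating damage.
; EndGrab only clears that timer and detaches, without restoring control, movement or the grab flag.
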(event OnComponentBeginOverlap(LungeHitbox)
  (params (OverlappedComponent :type Primitive%20Component%20Object%20Reference) (OtherActor :type Actor%20Object%20Reference) (OtherComp :type Primitive%20Component%20Object%20Reference) (OtherBodyIndex :type Integer) (bFromSweep :type Boolean) (SweepResult :type Hit%20Result%20Structure%20%28by%20ref%29))
  (if (and (Variables|Default|GetbIsLunging) (not (Variables|Default|GetbIsGrabbing)))
    (bind _asbp_pbplayer_character (Utilities|Casting|CastToBP_PBPlayerCharacter OtherActor))
    (CallFunction|InitiateGrab _asbp_pbplayer_character)))

(event Custom|StartLunge
  (Variables|Default|SetbIsLunging true)
  (Variables|Default|SetCurrentLungeRotation (Transformation|GetActorRotation))
  (Variables|/Script/Engine.CharacterMovementComponent|SetMaxWalkSpeed (Variables|Character|GetCharacterMovement) (* (Variables|Default|GetNormalMaxWalkSpeed) (Variables|Default|GetLungeSpeedMultiplier)))
  (Collision|SetCollisionEnabled (Variables|Default|GetLungeHitbox) "QueryOnly"))

(event Custom|EndLunge
  (bind _charactermovement (Variables|Character|GetCharacterMovement))
  (if (not (Variables|Default|GetbIsGrabbing))
    (Variables|Default|SetbIsLunging false)
    (Variables|/Script/Engine.CharacterMovementComponent|SetMaxWalkSpeed _charactermovement (Variables|Default|GetNormalMaxWalkSpeed))
    (Variables|/Script/Engine.CharacterMovementComponent|SetRotationRate _charactermovement (Variables|Default|GetNormalRotationRate))
    (Collision|SetCollisionEnabled (Variables|Default|GetLungeHitbox) "NoCollision")
    (Default|CallOnLungeEnded)))

(event Custom|InitiateGrab
  (params (GrabbedPlayer :type BP%20PB%20Player%20Character%20Object%20Reference))
  (Development|PrintString "Grab Initiated")
  (Variables|Default|SetbIsGrabbing true)
  (Variables|Default|SetbIsLunging false)
  (Collision|SetCollisionEnabled (Variables|Default|GetLungeHitbox) "NoCollision")
  (Pawn|Components|CharacterMovement|SetMovementMode (Variables|Character|GetCharacterMovement) "MOVE_None" 0)
  (Default|DisablePlayerControl GrabbedPlayer)
  (Transformation|AttachActorToActor GrabbedPlayer self "GrabSocket" "KeepRelative" "KeepRelative" "KeepRelative" true)
  (Utilities|Time|SetTimerbyFunctionName 0 "ApplyGrabDamage" 0.5 true)
  (Utilities|Time|SetTimerbyFunctionName 0 "EndGrab" 3.0))

(event Custom|ApplyGrabDamage
  (bind _grabbedplayer (Variables|Default|GetGrabbedPlayer))
  (if (Utilities|IsValid _grabbedplayer)
    (Default|ReceiveDamage _grabbedplayer 15.0)))

(event Custom|EndGrab
  (Development|PrintString "Grab Ended")
  (Utilities|Time|ClearTimerbyFunctionName 0 "ApplyGrabDamage")
  (Transformation|DetachFromActor (Variables|Default|GetGrabbedPlayer) "KeepRelative" "KeepRelative" "KeepRelative"))

(event EventBeginPlay
  (Variables|Default|SetNormalRotationRate (Variables|/Script/Engine.CharacterMovementComponent|GetRotationRate (Variables|Character|GetCharacterMovement)))
  (Components|Sphere|SetSphereRadius (Variables|Default|GetLungeHitbox) (Variables|Default|GetLungeHitboxRadius) true))

(event EventTick
  (params (DeltaSeconds :type Float%20%28single-precision%29))
  (if (Variables|Default|GetbIsLunging)
    (bind _output_get (Variables|Default|SetCurrentLungeRotation (Math|Interpolation|RInterpTo (Variables|Default|GetCurrentLungeRotation) (Math|Conversions|RotationFromXVector (Math|Vector|Normalize (- (Transformation|GetActorLocation (Game|GetPlayerCharacter 0)) (Transformation|GetActorLocation)))) (Utilities|Time|GetWorldDeltaSeconds) (Variables|Default|GetMaxTurnRateDuringLunge))))
    (Pawn|Input|AddMovementInput (Math|Vector|GetForwardVector _output_get) 1.0 false)))

(event EventDamage
  (params (DamageAmount :type Float%20%28double-precision%29))
  (Default|TakeDamage (Variables|Default|GetBP_HealthComponent) DamageAmount))

(fn ConstructionScript)